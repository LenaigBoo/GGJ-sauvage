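; Boss dialogue Blueprint that shows one line of text on screen each time its Talk event fires.
; Talk increments TalkIndex, creates a widget and adds it to the viewport if UI is invalid, then sets TalkText from the DIalogue array.
; The index increments before the read and is checked with <= Length, so it can read one past the last entry.
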(event EventTalk
  (Math|Integer|IncrementInt (Variables|Default|GetTalkIndex)
    (:%20%20
      (if (<= (Variables|Default|GetTalkIndex) (Utilities|Array|Length (Variables|Default|GetDIalogue)))
        (Variables|Default|GetUI
          (:then
            _)
          (:else
            (bind _returnvalue (UserInterface|CreateWidget 0 (Game|GetPlayerController 0)))
            (bind _output_get (Variables|Default|SetUI 0 _returnvalue))
            (UserInterface|Viewport|AddtoViewport _output_get 0)))
        (Rendering|Components|TextRender|SetText (Variables|Default|GetTalkText (.UI (Variables|Default|GetUI))) (Utilities|Text|ToText(String) (Utilities|Array|Get(acopy) (Variables|Default|GetDIalogue) (Variables|Default|GetTalkIndex))))))))

(fn ConstructionScript)