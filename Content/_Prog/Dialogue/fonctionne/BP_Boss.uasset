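; BP_Boss is a boss Blueprint that shows timed dialogue on screen through its Talk event.
; Talk reads the "Dial1" data table row, creates a UI widget and splits the row's map into lines (keys) and durations (values).
; A Delay loop displays each line for its duration and increments TalkIndex, with no end check.
; Older array-based dialogue and index-limit logic remains disconnected.
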(event EventTalk
  (bind _talkindex (Variables|Default|GetTalkIndex))
  (bind _returnvalue (Utilities|GetDataTableRow 0 "Dial1")
    (:then
      (bind _returnvalue_2 (UserInterface|CreateWidget 0))
      (bind _output_get (Variables|Default|SetUI 0 _returnvalue_2))
      (UserInterface|Viewport|AddtoViewport _output_get 0)
      (bind _keys (Utilities|Map|Keys (Utilities|Struct|Break _returnvalue)))
      (bind _values (Utilities|Map|Values (Utilities|Struct|Break _returnvalue)))
      (Rendering|Components|TextRender|SetText (Variables|Default|GetTalkText (.UI (Variables|Default|GetUI))) (Utilities|Text|ToText(String) (Utilities|Array|Get(acopy) _keys _talkindex)) :!label _label)
      (Utilities|FlowControl|Delay (Utilities|Array|Get(acopy) _values _talkindex))
      (bind _result (Math|Integer|IncrementInt _talkindex)
        (:%20%20
          (goto _label))))))

(fn ConstructionScript)